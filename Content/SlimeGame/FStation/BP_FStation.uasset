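; BP_FStation is a station in the slime game that collects biomaterial and shows its stock on a widget.
; BeginPlay resets the widget's progress bar and count text, then starts a timeline that endlessly ping-pongs the Fbuilding mesh's "Key 1" morph target with short pauses.
; AcceptBiomaterial adds to the count while below the maximum, without clamping, and refreshes the text, but always sets the progress bar to zero.
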(event EventBeginPlay
  (Utilities|FlowControl|Sequence
    (:then_0
      (bind _aswbp_fstation (Utilities|Casting|CastToWBP_FStation (UserInterface|GetUserWidgetObject (Variables|Default|GetWidget))))
      (Progress|SetPercent (Variables|/Game/SlimeGame/FStation/WBP_FStation.WBP_FStation_C|GetProgressBar_0 _aswbp_fstation) 0.0)
      (Variables|/Script/UMG.TextBlock|SetText (Variables|/Game/SlimeGame/FStation/WBP_FStation.WBP_FStation_C|GetTextBlock _aswbp_fstation) "0 / 1"))
    (:then_1
      ;[1 1 1] Looping animation of morph targets of the mesh
      (bind (_direction _newtrack_0) (Timeline|Timeline Play)
        (:Update
          (Components|SkeletalMesh|SetMorphTarget (Variables|Default|Getfbuilding) "Key 1" _newtrack_0 true))
        (:Finished
          (if (Utilities|Enum|Equal(Enum) _direction "Backward")
            (Utilities|FlowControl|Delay 0.2)
            (Timeline|Timeline PlayFromStart)
            (else
              (Utilities|FlowControl|Delay 0.2)
              (Timeline|Timeline ReverseFromEnd))))))))

(fn ConstructionScript)

(fn AcceptBiomaterial
  (params (Count :type Integer))
  (if (< (Variables|Default|GetBiomaterialCount) (Variables|Default|GetMaxBioCount))
    (bind _output_get (Variables|Default|SetBiomaterialCount (+ Count (Variables|Default|GetBiomaterialCount))))
    (bind _aswbp_fstation (Utilities|Casting|CastToWBP_FStation (UserInterface|GetUserWidgetObject (Variables|Default|GetWidget))))
    (Progress|SetPercent (Variables|/Game/SlimeGame/FStation/WBP_FStation.WBP_FStation_C|GetProgressBar_0 _aswbp_fstation) 0.0)
    (Variables|/Script/UMG.TextBlock|SetText (Variables|/Game/SlimeGame/FStation/WBP_FStation.WBP_FStation_C|GetTextBlock _aswbp_fstation) (Utilities|Text|ToText(String) (Utilities|String|Append (Utilities|String|ToString(Integer) _output_get) "/" (Utilities|String|ToString(Integer) (Variables|Default|GetMaxBioCount)))))))