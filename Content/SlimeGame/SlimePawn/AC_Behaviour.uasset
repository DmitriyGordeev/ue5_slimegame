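; Behaviour component for slime pawns that decides where the owning slime jumps on each Update.
; A slime carrying a resource targets and jumps to its Building; otherwise it jumps to its current target.
; With no valid target, or when the target is still a building, it searches by jumping randomly, biased toward the resource center when one is set.
; Search directions add the slime's FromOthers vector.
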(event EventBeginPlay
  (bind _asslime_pawn_parent (Utilities|Casting|CastToSlimePawnParent (Components|GetOwner)))
  (Variables|Default|SetOwningSlime _asslime_pawn_parent))

(fn SearchCycle
  (params (FromOthers :type Vector%202D%20Structure))
  (if (== (Math|Vector|VectorLength (Variables|/Game/SlimeGame/SlimePawn/SlimePawnParent.SlimePawnParent_C|GetResourceCenter (Variables|Default|GetOwningSlime))) 0.0)
    (Default|JumpinDirection (Variables|Default|GetOwningSlime) (+ (Math|Vector2D|MakeVector2D (Math|Random|RandomFloatinRange -1.0 1.0) (Math|Random|RandomFloatinRange -1.0 1.0)) FromOthers) 1.0 1.0)
    (else
      (bind _direction (CallFunction|DirtoResourceCenter FromOthers))
      (Default|JumpinDirection (Variables|Default|GetOwningSlime) _direction 1.0 1.0))))

(fn MovetoBuilding
  (bind _owningslime (Variables|Default|GetOwningSlime))
  (bind _building (Variables|/Game/SlimeGame/SlimePawn/SlimePawnParent.SlimePawnParent_C|GetBuilding _owningslime))
  (Utilities|IsValid _building
    (:Is%20Valid
      (Variables|/Game/SlimeGame/SlimePawn/SlimePawnParent.SlimePawnParent_C|SetCurrentTarget _owningslime _building)
      (Default|JumptoActor _owningslime _building))))

(fn Update
  (bind _owningslime (Variables|Default|GetOwningSlime))
  (bind _currenttarget (Variables|/Game/SlimeGame/SlimePawn/SlimePawnParent.SlimePawnParent_C|GetCurrentTarget _owningslime))
  (if (Variables|/Game/SlimeGame/SlimePawn/SlimePawnParent.SlimePawnParent_C|GetIsCarryingResource _owningslime)
    (CallFunction|MovetoBuilding)
    (else
      ;[1 1 1] If Slime is not carrying resource and CurrentTarget is BP_Building we need to pick new direction (next block), otherwise will stuck, jumping towards building
      (Utilities|Casting|CastToBP_Building _currenttarget
        (:then
          (CallFunction|SearchCycle (Variables|/Game/SlimeGame/SlimePawn/SlimePawnParent.SlimePawnParent_C|GetFromOthers (Variables|Default|GetOwningSlime)) :!label _label))
        (:CastFailed
          (if (Utilities|IsValid _currenttarget)
            (Default|JumptoActor (Variables|Default|GetOwningSlime) _currenttarget)
            (else
              (goto _label))))))))

(fn DirtoResourceCenter
  (params (FromOthers :type Vector%202D%20Structure))
  (bind _owningslime (Variables|Default|GetOwningSlime))
  (bind _staticmesh (Variables|/Game/SlimeGame/SlimePawn/SlimePawnParent.SlimePawnParent_C|GetStaticMesh _owningslime))
  (bind _resourcecenter (Variables|/Game/SlimeGame/SlimePawn/SlimePawnParent.SlimePawnParent_C|GetResourceCenter _owningslime))
  (bind _returnvalue (Transformation|GetWorldLocation _staticmesh))
  (bind _returnvalue_2 (- _resourcecenter _returnvalue))
  (bind _returnvalue_3 (Math|Vector|Normalize _returnvalue_2))
  (bind (_x _y) (Class|KismetMathLibrary|BreakVector3f _returnvalue_3))
  (return (+ (+ (Math|Vector2D|MakeVector2D _x _y) FromOthers) (Math|Vector2D|MakeVector2D (Math|Random|RandomFloatinRange -1.0 1.0) (Math|Random|RandomFloatinRange -1.0 1.0)))))