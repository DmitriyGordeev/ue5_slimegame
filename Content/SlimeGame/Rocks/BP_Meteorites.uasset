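; Decorative meteorite field actor that scatters randomized rock meshes around its origin and slowly spins as a whole.
; The construction script adds Amount static mesh components, each from one of three randomly picked branches with identical transform logic.
; Transforms combine cosine/sine offsets within radius bounds, random height, random rotation and non-uniform scale.
; Tick yaws the whole actor at RotationRate scaled by delta time.
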(event EventTick
  (params (DeltaSeconds :type Float%20%28single-precision%29))
  (Class|Actor|AddActorWorldRotation (Math|Rotator|MakeRotator 0.0 0.0 (* DeltaSeconds (Variables|Default|GetRotationRate)))))

(fn ConstructionScript
  (bind _returnvalue (Math|Random|RandomRotator true))
  (bind _returnvalue_2 (Math|Random|RandomFloatinRange 0.0 359.0))
  (bind _minradius (Variables|Default|GetMinRadius))
  (bind _maxradius (Variables|Default|GetMaxRadius))
  (bind _minheight (Variables|Default|GetMinHeight))
  (bind _maxheight (Variables|Default|GetMaxHeight))
  (bind _maxscale (Variables|Default|GetMaxScale))
  (bind _minscale (Variables|Default|GetMinScale))
  (bind _returnvalue_3 (Math|Random|RandomFloatinRange _minscale _maxscale))
  (bind _returnvalue_4 (Math|Conversions|ToFloat(Integer) _minradius))
  (bind _returnvalue_5 (Math|Conversions|ToFloat(Integer) _maxradius))
  (bind _returnvalue_6 (Math|Conversions|ToFloat(Integer) _minheight))
  (bind _returnvalue_7 (Math|Conversions|ToFloat(Integer) _maxheight))
  (bind _returnvalue_8 (Math|Trig|Cos(Degrees) _returnvalue_2))
  (bind _returnvalue_9 (Math|Trig|Sin(Degrees) _returnvalue_2))
  (bind _returnvalue_10 (Math|Vector|MakeVector _returnvalue_3 _returnvalue_3 _returnvalue_3))
  (bind _returnvalue_11 (Math|Random|RandomFloatinRange _returnvalue_6 _returnvalue_7))
  (bind _returnvalue_12 (Math|Random|RandomFloatinRange _returnvalue_4 _returnvalue_5))
  (bind _returnvalue_13 (* _returnvalue_12 _returnvalue_8))
  (bind _returnvalue_14 (* _returnvalue_12 _returnvalue_9))
  (bind _returnvalue_15 (Math|Vector|MakeVector _returnvalue_13 _returnvalue_14 _returnvalue_11))
  (bind _returnvalue_16 (Math|Transform|MakeTransform _returnvalue_15 _returnvalue _returnvalue_10))
  (for _index (range 0 (- (Variables|Default|GetAmount) 1))
    (switch int (Math|Random|RandomInteger 3)
      (:0
        (AddComponent|AddStaticMeshComponent false _returnvalue_16))
      (:1
        (AddComponent|AddStaticMeshComponent false _returnvalue_16))
      (:2
        (AddComponent|AddStaticMeshComponent false _returnvalue_16)))))