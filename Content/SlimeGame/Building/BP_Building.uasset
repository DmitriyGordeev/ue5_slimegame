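; Building that collects resources delivered by green slimes and shows progress on a widget bar.
; A looping one-second timer designates a random SlimePawn_Green for gathering whenever none is assigned, binding to its arrival and destruction dispatchers.
; Arrival increments the resource count, refreshes the widget against the maximum and frees the slot for the next pick.
; Destruction of the designated slime also frees the slot.
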(event Custom|DesignateSlime
  (if (not (Variables|Default|GetHasDesignated))
    ;[1 1 1] pick random slime to designate and bind to it's events
    (bind _outactors (Actor|GetAllActorsOfClass "/Game/SlimeGame/SlimePawn/SlimePawn_Green.SlimePawn_Green_C"))
    (bind _output_get (Variables|Default|SetDesignatedSlime (.OutItem (Utilities|Array|Random _outactors))))
    (EventDispatchers|BindEventtoEDSlimeDestroyed _output_get (delegate Custom|OnDesignatedSlimeDestroyed))
    (EventDispatchers|BindEventtoEDSlimeArrivedtoBuilding _output_get (delegate Custom|OnSlimeArrived))
    (Variables|/Game/SlimeGame/SlimePawn/SlimePawnParent.SlimePawnParent_C|SetDesignatedForGathering (Variables|Default|GetDesignatedSlime) true)
    (Variables|Default|SetHasDesignated true)
    (Development|PrintString (Utilities|String|Append "Designating slime = " (Utilities|String|ToString(Integer) 0)))))

(event Custom|OnDesignatedSlimeDestroyed
  ;[1 1 1] Ставим HasDesinated = false, если слайма, несущего ресурс, уничтожили
  (Development|PrintString "Designated Slime Destroyed")
  (Variables|Default|SetHasDesignated false))

(event Custom|OnSlimeArrived
  (bind _designatedslime (Variables|Default|GetDesignatedSlime))
  ;[1 1 1] Когда слайм приносит ресурс
  (Development|PrintString "Accept resource")
  (Variables|Default|SetResourceCount (+ (Variables|Default|GetResourceCount) 1))
  (Variables|Default|SetHasDesignated false)
  (Utilities|IsValid (Variables|Default|GetProgressBarWidget)
    (:Is%20Valid
      (CallFunction|UpdateWidget))
    (:Is%20Not%20Valid
      _))
  (Utilities|IsValid _designatedslime
    (:Is%20Valid
      (EventDispatchers|UnbindallEventsfromEDSlimeArrivedtoBuilding _designatedslime)
      (EventDispatchers|UnbindallEventsfromOnDestroyed _designatedslime)
      ;[1 1 1] Debug
      (Development|PrintString (Utilities|String|Append "Collected = " (Utilities|String|ToString(Integer) (Variables|Default|GetResourceCount))))
      (Development|PrintString (Utilities|String|Append "HasDesignated" (Utilities|String|ToString(Boolean) (Variables|Default|GetHasDesignated)))))))

(event EventBeginPlay
  (Utilities|FlowControl|Sequence
    (:then_0
      (bind _aswbp_building_progress (Utilities|Casting|CastToWBP_BuildingProgress (UserInterface|GetUserWidgetObject (Variables|Default|GetResourceWidget))))
      (Variables|Default|SetProgressBarWidget _aswbp_building_progress)
      (CallFunction|UpdateWidget))
    (:then_1
      (Utilities|Time|SetTimerbyEvent (delegate Custom|DesignateSlime) 1.0 true))))

(fn ConstructionScript)

(fn UpdateWidget
  (bind _resourcecount (Variables|Default|GetResourceCount))
  (bind _progressbarwidget (Variables|Default|GetProgressBarWidget))
  (Variables|/Script/UMG.TextBlock|SetText (Variables|/Game/SlimeGame/Building/WBP_BuildingProgress.WBP_BuildingProgress_C|GetProgressText _progressbarwidget) (Utilities|Text|ToText(Integer) _resourcecount))
  (Progress|SetPercent (Variables|/Game/SlimeGame/Building/WBP_BuildingProgress.WBP_BuildingProgress_C|GetResourceBar _progressbarwidget) (/ (Math|Conversions|ToFloat(Integer) _resourcecount) (Variables|Default|GetMaxResource))))