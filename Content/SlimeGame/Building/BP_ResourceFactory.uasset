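; BP_ResourceFactory is a building actor that periodically spawns BP_ResourceItem pickups around itself.
; BeginPlay starts a looping timer that fires SpawnResourceItem every few seconds.
; Each spawn offsets the item horizontally from the root's world location using a random angle and a random radius capped by MaxRadius, converted with cosine and sine.
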(event Custom|Spawn%20Resource%20Item
  (bind _returnvalue (Math|Random|RandomInteger 360))
  (bind _maxradius (Variables|Default|GetMaxRadius))
  (bind _returnvalue_2 (Math|Random|RandomFloatinRange 1.0 _maxradius))
  (Game|SpawnActorfromClass "/Game/SlimeGame/Building/BP_ResourceItem.BP_ResourceItem_C" (Math|Transform|MakeTransform (+ (Transformation|GetWorldLocation (Variables|Default|GetDefaultSceneRoot)) (Math|Vector|MakeVector (* _returnvalue_2 (Math|Trig|Cos(Degrees) (Math|Conversions|ToFloat(Integer) _returnvalue))) (* _returnvalue_2 (Math|Trig|Sin(Degrees) (Math|Conversions|ToFloat(Integer) _returnvalue))) 0.0))) "Undefined" 0 0))

(event EventBeginPlay
  (Utilities|Time|SetTimerbyEvent (delegate Custom|Spawn%20Resource%20Item) 5.0 true))

(fn ConstructionScript)