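; Main menu game mode that shows the starting screen and applies saved audio settings on BeginPlay.
; It adds WBP_MainMenuStartingScreen to the viewport with Game and UI input and a visible cursor.
; It then loads the custom settings save and applies its volume to the Master sound class through a sound mix.
; A missing save is created with defaults; one that fails the cast is deleted and recreated.
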(event EventBeginPlay
  (bind _returnvalue (Game|GetPlayerController 0))
  (Utilities|FlowControl|Sequence
    (:then_0
      (bind _returnvalue_2 (UserInterface|CreateWidget "/Game/Shared/MainMenuFiles/WBP_MainMenuStartingScreen.WBP_MainMenuStartingScreen_C" _returnvalue))
      (UserInterface|Viewport|AddtoViewport _returnvalue_2 0)
      (Input|SetInputModeGameandUI _returnvalue _returnvalue_2 "DoNotLock" true false)
      (Variables|/Script/Engine.PlayerController|SetbShowMouseCursor _returnvalue true))
    (:then_1
      (bind _returnvalue_3 (SaveGame|DoesSaveGameExist "SavedCustomSettingValues"))
      (if _returnvalue_3
        (bind _returnvalue_4 (SaveGame|LoadGamefromSlot "SavedCustomSettingValues"))
        (bind _asmy_custom_settings_save (Utilities|Casting|CastToMyCustomSettingsSave _returnvalue_4)
          (:then
            (Audio|SetSoundMixClassOverride "/Game/Shared/MainMenuFiles/MasterSoundmixClass.MasterSoundmixClass" "/Engine/EngineSounds/Master.Master" (Variables|/Game/Shared/MainMenuFiles/MyCustomSettingsSave.MyCustomSettingsSave_C|GetVolume _asmy_custom_settings_save) 1.0 0.0 true)
            (Audio|PushSoundMixModifier "/Game/Shared/MainMenuFiles/MasterSoundmixClass.MasterSoundmixClass"))
          (:CastFailed
            ;[1 1 1] Если сейв не кастится он все равно не сможет быть использован в дальнейшем. Лучше сразу пересоздвть
            (SaveGame|DeleteGameinSlot "SavedCustomSettingValues")
            (bind _returnvalue_5 (SaveGame|CreateSaveGameObject "/Game/Shared/MainMenuFiles/MyCustomSettingsSave.MyCustomSettingsSave_C" :!label _label))
            (SaveGame|SaveGametoSlot _returnvalue_5 "SavedCustomSettingValues")))
        (else
          (goto _label))))))

(fn ConstructionScript)